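; Player controller for testing Advance Replay recording and playback.
; On BeginPlay it shows the WBP_PlayMenu widget.
; Debug keys 1, 2 and 3 print a message, then call the AdvanceReplaySubsystem to start recording, stop recording or play back a replay under one hardcoded test name.
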(event EventBeginPlay
  (|CallParentFunction)
  (Class|AdvanceReplayPlayerController|ShowMenuWidgetClass "/Game/Widgets/WBP_PlayMenu.WBP_PlayMenu_C"))

(event EventTick
  (params (DeltaSeconds :type Float%20%28single-precision%29))
  (|CallParentFunction DeltaSeconds))

(event Input|KeyboardEvents|1
  (params (Key :type Key%20Structure :default "None"))
  (:Pressed
    (Development|PrintString "START RECORD REPLAY" true true "(R=0.342294,G=1.000000,B=0.000000,A=1.000000)" 1e+01)
    (Class|AdvanceReplaySubsystem|StartRecordReplay (Subsystems|GetAdvanceReplaySubsystem) "TestReplay")))

(event Input|KeyboardEvents|2
  (params (Key :type Key%20Structure :default "None"))
  (:Pressed
    (Development|PrintString "STOP RECORD REPLAY" true true "(R=1.000000,G=0.044383,B=0.000000,A=1.000000)" 1e+01)
    (Class|AdvanceReplaySubsystem|StopRecordReplay (Subsystems|GetAdvanceReplaySubsystem))))

(event Input|KeyboardEvents|3
  (params (Key :type Key%20Structure :default "None"))
  (:Pressed
    (Development|PrintString "PLAY LAST REPLAY" true true "(R=0.863357,G=1.000000,B=0.000000,A=1.000000)" 1e+01)
    (Class|AdvanceReplaySubsystem|StartPlayReplay (Subsystems|GetAdvanceReplaySubsystem) "TestReplay")))

(fn ConstructionScript
  (|CallParentFunction))