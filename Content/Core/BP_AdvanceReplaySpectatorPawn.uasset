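; BP_AdvanceReplaySpectatorPawn is a replay spectator pawn that follows an off-road car with a spring-arm camera.
; On BeginPlay it takes the first OffroadCar_Pawn found in the level as its target.
; Each Tick it smoothly interpolates its location toward that vehicle while the reference is valid.
; Keys 1 and 2 switch between two view presets by setting the spring arm's length, rotation and offset.
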(event EventBeginPlay
  (bind _outactors (Actor|GetAllActorsOfClass "/Game/External/VehicleTemplate/Blueprints/OffroadCar/OffroadCar_Pawn.OffroadCar_Pawn_C"))
  (Variables|Default|SetVehicle (Utilities|Array|Get(acopy) _outactors)))

(event EventTick
  (params (DeltaSeconds :type Float%20%28single-precision%29))
  (bind _vehicle (Variables|Default|GetVehicle))
  (Utilities|IsValid _vehicle
    (:Is%20Valid
      (Transformation|SetActorLocation (Math|Interpolation|VInterpTo (Transformation|GetActorLocation) (Transformation|GetActorLocation _vehicle) DeltaSeconds 1e+01) false false))))

(event Input|KeyboardEvents|1
  (params (Key :type Key%20Structure :default "None"))
  (bind _springarm (Variables|Default|GetSpringArm))
  (:Pressed
    (Variables|/Script/Engine.SpringArmComponent|SetTargetArmLength _springarm 1.2e+03)
    (Transformation|SetRelativeRotation _springarm "-20.000000,0.000000,0.000000" false false)
    (Transformation|SetRelativeLocation _springarm "0.000000,0.000000,0.000000" false false)))

(event Input|KeyboardEvents|2
  (params (Key :type Key%20Structure :default "None"))
  (bind _springarm (Variables|Default|GetSpringArm))
  (:Pressed
    (Variables|/Script/Engine.SpringArmComponent|SetTargetArmLength _springarm 1.5e+03)
    (Transformation|SetRelativeRotation _springarm "-20.000000,-90.000000,0.000000" false false)
    (Transformation|SetRelativeLocation _springarm "500.000000,0.000000,0.000000" false false)))

(fn ConstructionScript)